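; BP_CdRom is a CD-ROM problem actor, derived from a parent class, that can show an intact or broken state.
; The construction script runs the parent's script, sets ProblemType to the BrokenCdRom enum value and hides the Broken component.
; Every Tick, the ActorState boolean toggles visibility between StaticMesh when true and Broken when false, polling the state rather than reacting to changes.
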(event EventBeginPlay)

(event Collision|EventActorBeginOverlap
  (params (OtherActor :type Actor%20Object%20Reference)))

(event EventTick
  (params (DeltaSeconds :type Float%20%28single-precision%29))
  (bind _actorstate (Variables|Default|GetActorState))
  (Rendering|SetVisibility (Variables|Default|Getbroken) (not _actorstate) false)
  (Rendering|SetVisibility (Variables|Default|GetStaticMesh) _actorstate false))

(fn ConstructionScript
  (|CallParentFunction)
  (Variables|Default|SetProblemType (Math|Conversions|ToInteger(Byte) (Utilities|Enum|LiteralenumE_ProblemType "VE_BrokenCdRom")))
  (Rendering|SetVisibility (Variables|Default|Getbroken) false false))