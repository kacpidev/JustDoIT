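; Corporation manager for the JustDoIT game, turning total money earned into escalating alarm feedback and ending the game when money goes negative.
; Tick pushes game time to the HUD and maps money thresholds to an error level, crossfading alarm or Gandalf audio on each change.
; Lowest level pulses four lights with squared sine; top levels toggle the workplaces' movie material parameter.
; EndGame fixes workplaces, shows the cursor, disables pawn input and destroys itself.
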(event Custom|EndGame
  (bind _returnvalue (Game|GetPlayerController 0))
  (bind _outactors (Actor|GetAllActorsOfClass "/Game/JustDoIT/Blueprints/BP_JustDoITWorkplace.BP_JustDoITWorkplace_C"))
  (for _array_element _outactors
    (Default|Fix _array_element)
    (Variables|/Script/Engine.PlayerController|SetbShowMouseCursor _returnvalue true)
    (Input|DisableInput (Pawn|GetControlledPawn _returnvalue) _returnvalue)
    (Actor|DestroyActor)))

(event EventBeginPlay
  (bind _gandalf (Variables|Default|Getgandalf))
  (Audio|Components|Audio|Play (Variables|Default|Getal_1) 0.0)
  (Audio|Components|Audio|FadeOut (Variables|Default|Getal_1) 0.0 0.0 :!class /Script/Engine.AudioComponent)
  (Audio|Components|Audio|Play (Variables|Default|Getal_2) 0.0)
  (Audio|Components|Audio|FadeOut (Variables|Default|Getal_2) 0.0 0.0 :!class /Script/Engine.AudioComponent)
  (Audio|Components|Audio|Play (Variables|Default|Getal_3) 0.0)
  (Audio|Components|Audio|FadeOut (Variables|Default|Getal_3) 0.0 0.0 :!class /Script/Engine.AudioComponent)
  (Audio|Components|Audio|Play (Variables|Default|Getal_4) 0.0)
  (Audio|Components|Audio|FadeOut (Variables|Default|Getal_4) 0.0 0.0 :!class /Script/Engine.AudioComponent)
  (Audio|Components|Audio|Play _gandalf 0.0)
  (Audio|Components|Audio|FadeOut _gandalf 0.0 0.0 :!class /Script/Engine.AudioComponent)
  (Variables|Default|SetoldErrLvl 199)
  (Variables|Default|SeterrLvl 84)
  (bind _outactors (Actor|GetAllActorsOfClass "/Game/JustDoIT/Blueprints/BP_JustDoITWorkplace.BP_JustDoITWorkplace_C"))
  (Variables|Default|SetWorkplacesVector _outactors))

(event Collision|EventActorBeginOverlap
  (params (OtherActor :type Actor%20Object%20Reference)))

(event EventTick
  (params (DeltaSeconds :type Float%20%28single-precision%29))
  (bind _returnvalue (Utilities|Time|GetRealTimeSeconds))
  (bind _totalmoneyearned (Variables|Default|GetTotalMoneyEarned))
  (bind _returnvalue_2 (* _returnvalue 3.0))
  (bind _returnvalue_3 (Math|Trig|Sin(Radians) _returnvalue_2))
  (bind _returnvalue_4 (Math|Float|Power _returnvalue_3 2.0))
  (bind _returnvalue_5 (* _returnvalue_4 1e+05))
  (if (< _totalmoneyearned 0.0)
    (CallFunction|EndGame)
    (else
      (Variables|Default|SetGameTime (+ DeltaSeconds (Variables|Default|GetGameTime)))
      (bind _asjust_do_ithud (Utilities|Casting|CastToJustDoITHUD (HUD|GetHUD (Game|GetPlayerController 0))))
      (Variables|/Script/JustDoIT.JustDoITHUD|SetGameTime _asjust_do_ithud (Variables|Default|GetGameTime))
      (if (< _totalmoneyearned 1.5e+03)
        (bind _output_get (Variables|Default|SeterrLvl 3))
        (Utilities|FlowControl|Sequence
          (:then_0
            (Rendering|Components|Light|SetIntensity (Variables|Default|GetPointLight) _returnvalue_5)
            (Rendering|Components|Light|SetIntensity (Variables|Default|GetPointLight1) _returnvalue_5)
            (Rendering|Components|Light|SetIntensity (Variables|Default|GetPointLight2) _returnvalue_5)
            (Rendering|Components|Light|SetIntensity (Variables|Default|GetPointLight3) _returnvalue_5))
          (:then_1
            (if (!= _output_get (Variables|Default|GetoldErrLvl))
              (CallFunction|PlaySample _output_get)
              (Variables|Default|SetoldErrLvl _output_get))))
        (else
          (Utilities|FlowControl|Sequence
            (:then_0
              (if (< _totalmoneyearned 3e+03)
                (bind _output_get_2 (Variables|Default|SeterrLvl 2))
                (if (!= _output_get_2 (Variables|Default|GetoldErrLvl))
                  (CallFunction|PlaySample _output_get_2)
                  (Variables|Default|SetoldErrLvl _output_get_2))
                (elif (< _totalmoneyearned 4.5e+03)
                  (bind _output_get_3 (Variables|Default|SeterrLvl 1))
                  (if (!= _output_get_3 (Variables|Default|GetoldErrLvl))
                    (CallFunction|PlaySample _output_get_3)
                    (Variables|Default|SetoldErrLvl _output_get_3))
                  (elif (< _totalmoneyearned 6e+03)
                    (bind _output_get_4 (Variables|Default|SeterrLvl 0))
                    (if (!= _output_get_4 (Variables|Default|GetoldErrLvl))
                      (CallFunction|PlaySample _output_get_4)
                      (bind _outactors (Actor|GetAllActorsOfClass "/Game/JustDoIT/Blueprints/BP_JustDoITWorkplace.BP_JustDoITWorkplace_C"))
                      (for _array_element _outactors
                        (Rendering|Material|SetScalarParameterValue (Variables|/Game/JustDoIT/Blueprints/BP_JustDoITWorkplace.BP_JustDoITWorkplace_C|GetMaterialInstance _array_element) "playMovie" 0.0 :!class /Script/Engine.MaterialInstanceDynamic))
                      (Variables|Default|SetoldErrLvl _output_get_4))
                    (else
                      (bind _output_get_5 (Variables|Default|SeterrLvl -1))
                      (if (!= _output_get_5 (Variables|Default|GetoldErrLvl))
                        (CallFunction|PlaySample _output_get_5)
                        (bind _outactors_2 (Actor|GetAllActorsOfClass "/Game/JustDoIT/Blueprints/BP_JustDoITWorkplace.BP_JustDoITWorkplace_C"))
                        (for _array_element_2 _outactors_2
                          (Rendering|Material|SetScalarParameterValue (Variables|/Game/JustDoIT/Blueprints/BP_JustDoITWorkplace.BP_JustDoITWorkplace_C|GetMaterialInstance _array_element_2) "playMovie" 1.0 :!class /Script/Engine.MaterialInstanceDynamic)
                          (Variables|Default|SetoldErrLvl _output_get_5))))))))
            (:then_1
              (Rendering|Components|Light|SetIntensity (Variables|Default|GetPointLight) 0.0)
              (Rendering|Components|Light|SetIntensity (Variables|Default|GetPointLight1) 0.0)
              (Rendering|Components|Light|SetIntensity (Variables|Default|GetPointLight2) 0.0)
              (Rendering|Components|Light|SetIntensity (Variables|Default|GetPointLight3) 0.0))))))))

(fn ConstructionScript
  (Media|MediaPlayer|Play (Variables|Default|GetMediaPlayer) :!class /Script/MediaAssets.MediaPlayer))

(fn PlaySample
  (params (SampleNr :type Integer))
  (bind _gandalf (Variables|Default|Getgandalf))
  (bind _al_2 (Variables|Default|Getal_2))
  (bind _al_3 (Variables|Default|Getal_3))
  (bind _al_4 (Variables|Default|Getal_4))
  (bind _al_1 (Variables|Default|Getal_1))
  (switch int SampleNr
    (:-1
      (Utilities|FlowControl|Sequence
        (:then_0
          (Audio|Components|Audio|FadeOut _al_1 1.0 0.0 :!class /Script/Engine.AudioComponent :!label _label))
        (:then_1
          (Audio|Components|Audio|FadeIn _gandalf 1.0 1.0 0.0 :!class /Script/Engine.AudioComponent))))
    (:0
      (Utilities|FlowControl|Sequence
        (:then_0
          (Audio|Components|Audio|FadeOut _al_2 1.0 0.0 :!class /Script/Engine.AudioComponent :!label _label_2))
        (:then_1
          (Audio|Components|Audio|FadeOut _gandalf 1.0 0.0 :!class /Script/Engine.AudioComponent :!label _label_3))
        (:then_2
          (Audio|Components|Audio|FadeIn _al_1 1.0 1.0 0.0 :!class /Script/Engine.AudioComponent))))
    (:1
      (Utilities|FlowControl|Sequence
        (:then_0
          (goto _label))
        (:then_1
          (Audio|Components|Audio|FadeOut _al_3 1.0 0.0 :!class /Script/Engine.AudioComponent :!label _label_4))
        (:then_2
          (Audio|Components|Audio|FadeIn _al_2 1.0 1.0 0.0 :!class /Script/Engine.AudioComponent))))
    (:2
      (Utilities|FlowControl|Sequence
        (:then_0
          (goto _label_2))
        (:then_1
          (Audio|Components|Audio|FadeOut _al_4 1.0 0.0 :!class /Script/Engine.AudioComponent))
        (:then_2
          (Audio|Components|Audio|FadeIn _al_3 1.0 1.0 0.0 :!class /Script/Engine.AudioComponent))))
    (:3
      (Utilities|FlowControl|Sequence
        (:then_0
          (goto _label_4))
        (:then_1
          (goto _label_3))
        (:then_2
          (Audio|Components|Audio|FadeIn _al_4 1.0 1.0 0.0 :!class /Script/Engine.AudioComponent))))))