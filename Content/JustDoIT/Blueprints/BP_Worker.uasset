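; BP_Worker is a worker character that loops an animation on BeginPlay and randomizes its colors in the Construction Script.
; Dynamic instances of MI_Tie color material slots 2 and 5 from a tie palette, slot 0 from that palette multiplied by LightUp, and slot 4 from hair colors.
; Each pick is independent; the 0–4 range exceeds the four cases, so slot 0 can stay uncolored and skip hair setup, and hair can stay uncolored.
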(event EventBeginPlay
  (Components|Animation|PlayAnimation (Variables|Default|Getworker) "/Game/JustDoIT/Meshes/worker_Anim.worker_Anim" true))

(event Collision|EventActorBeginOverlap
  (params (OtherActor :type Actor%20Object%20Reference)))

(event EventTick
  (params (DeltaSeconds :type Float%20%28single-precision%29)))

(fn ConstructionScript
  (bind _worker (Variables|Default|Getworker))
  (bind _lightup (LocalVariables|GetLightUp))
  (bind _returnvalue (Math|Conversions|ToVector(LinearColor) _lightup))
  (bind _returnvalue_2 (Rendering|Material|CreateDynamicMaterialInstance "/Game/JustDoIT/Materials/MI_Tie.MI_Tie" :!class /Script/Engine.KismetMaterialLibrary))
  (Rendering|Material|SetMaterial _worker 2 _returnvalue_2)
  (Rendering|Material|SetMaterial _worker 5 _returnvalue_2)
  (switch int (Math|Random|RandomIntegerinRange 0 4)
    (:Default
      (Rendering|Material|SetVectorParameterValue _returnvalue_2 "Color" (LocalVariables|GetTie1) :!class /Script/Engine.MaterialInstanceDynamic :!label _label))
    (:0
      (goto _label))
    (:1
      (Rendering|Material|SetVectorParameterValue _returnvalue_2 "Color" (LocalVariables|GetTie2) :!class /Script/Engine.MaterialInstanceDynamic))
    (:2
      (Rendering|Material|SetVectorParameterValue _returnvalue_2 "Color" (LocalVariables|GetTie3) :!class /Script/Engine.MaterialInstanceDynamic))
    (:3
      (Rendering|Material|SetVectorParameterValue _returnvalue_2 "Color" (LocalVariables|GetTie4) :!class /Script/Engine.MaterialInstanceDynamic)))
  (bind _returnvalue_3 (Rendering|Material|CreateDynamicMaterialInstance "/Game/JustDoIT/Materials/MI_Tie.MI_Tie" :!class /Script/Engine.KismetMaterialLibrary))
  (Rendering|Material|SetMaterial (Variables|Default|Getworker) 0 _returnvalue_3)
  (switch int (Math|Random|RandomIntegerinRange 0 4)
    (:0
      (Rendering|Material|SetVectorParameterValue _returnvalue_3 "Color" (Math|Conversions|ToLinearColor(Vector) (* (Math|Conversions|ToVector(LinearColor) (LocalVariables|GetTie1)) _returnvalue)) :!class /Script/Engine.MaterialInstanceDynamic))
    (:1
      (Rendering|Material|SetVectorParameterValue _returnvalue_3 "Color" (Math|Conversions|ToLinearColor(Vector) (* _returnvalue (Math|Conversions|ToVector(LinearColor) (LocalVariables|GetTie2)))) :!class /Script/Engine.MaterialInstanceDynamic))
    (:2
      (Rendering|Material|SetVectorParameterValue _returnvalue_3 "Color" (Math|Conversions|ToLinearColor(Vector) (* _returnvalue (Math|Conversions|ToVector(LinearColor) (LocalVariables|GetTie3)))) :!class /Script/Engine.MaterialInstanceDynamic))
    (:3
      (Rendering|Material|SetVectorParameterValue _returnvalue_3 "Color" (Math|Conversions|ToLinearColor(Vector) (* _returnvalue (Math|Conversions|ToVector(LinearColor) (LocalVariables|GetTie4)))) :!class /Script/Engine.MaterialInstanceDynamic)))
  (bind _returnvalue_4 (Rendering|Material|CreateDynamicMaterialInstance "/Game/JustDoIT/Materials/MI_Tie.MI_Tie" :!class /Script/Engine.KismetMaterialLibrary))
  (Rendering|Material|SetMaterial (Variables|Default|Getworker) 4 _returnvalue_4)
  (switch int (Math|Random|RandomIntegerinRange 0 4)
    (:0
      (Rendering|Material|SetVectorParameterValue _returnvalue_4 "Color" (LocalVariables|GetHair1) :!class /Script/Engine.MaterialInstanceDynamic))
    (:1
      (Rendering|Material|SetVectorParameterValue _returnvalue_4 "Color" (LocalVariables|GetHair2) :!class /Script/Engine.MaterialInstanceDynamic))
    (:2
      (Rendering|Material|SetVectorParameterValue _returnvalue_4 "Color" (LocalVariables|GetHair3) :!class /Script/Engine.MaterialInstanceDynamic))
    (:3
      (Rendering|Material|SetVectorParameterValue _returnvalue_4 "Color" (LocalVariables|GetHair4) :!class /Script/Engine.MaterialInstanceDynamic))))