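; Janitor character that slowly patrols a loop of four waypoints while playing a looping animation.
; Waypoints are offsets from the spawn location recorded at BeginPlay, with movement driven by SimpleMoveToLocation on its controller.
; Tick reissues the move until the janitor nears the current goal, then identifies that waypoint by vector comparison and switches to the next, wrapping to the first.
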(event EventBeginPlay
  (Utilities|FlowControl|Sequence
    (:then_0
      (Components|Animation|PlayAnimation (Variables|Character|GetMesh) "/Game/JustDoIT/Meshes/janitor_Anim.janitor_Anim" true))
    (:then_1
      (Variables|Default|Setdestination (Variables|Default|Getdest1))
      (Variables|Default|Setstart (Transformation|GetActorLocation))
      (AI|Navigation|SimpleMovetoLocation (Pawn|GetController) (+ (Variables|Default|Getdestination) (Variables|Default|Getstart))))))

(event Collision|EventActorBeginOverlap
  (params (OtherActor :type Actor%20Object%20Reference)))

(event EventTick
  (params (DeltaSeconds :type Float%20%28single-precision%29))
  (bind _dest2 (Variables|Default|Getdest2))
  (bind _dest3 (Variables|Default|Getdest3))
  (bind _dest4 (Variables|Default|Getdest4))
  (Math|Float|CompareFloat (Math|Vector|VectorLength (- (+ (Variables|Default|Getdestination) (Variables|Default|Getstart)) (Transformation|GetActorLocation))) 2.2e+02
    (:>
      (AI|Navigation|SimpleMovetoLocation (Pawn|GetController) (+ (Variables|Default|Getdestination) (Variables|Default|Getstart)) :!label _label))
    (:==
      (goto _label))
    (:<
      (Math|Float|CompareFloat (Math|Vector|VectorLength (- (Variables|Default|Getdestination) (Variables|Default|Getdest1))) 1.0
        (:>
          (Math|Float|CompareFloat (Math|Vector|VectorLength (- (Variables|Default|Getdestination) _dest2)) 1.0
            (:>
              (Math|Float|CompareFloat (Math|Vector|VectorLength (- (Variables|Default|Getdestination) _dest3)) 1.0
                (:>
                  (Math|Float|CompareFloat (Math|Vector|VectorLength (- (Variables|Default|Getdestination) _dest4)) 1.0
                    (:<
                      (Variables|Default|Setdestination (Variables|Default|Getdest1)))))
                (:<
                  (Variables|Default|Setdestination _dest4))))
            (:<
              (Variables|Default|Setdestination _dest3))))
        (:<
          (Variables|Default|Setdestination _dest2))))))

(fn ConstructionScript
  (Variables|/Script/Engine.CharacterMovementComponent|SetMaxWalkSpeed (Variables|Character|GetCharacterMovement) 1e+02))