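; BP_StockDisplay is an actor that visualizes the corporation's earnings as a particle system at a height or position along a line.
; BeginPlay caches the first BP_JustDoITCorporation found in the level.
; Every Tick, it places the particle system between Bottom and Top by TotalMoneyEarned over a fixed target, without clamping.
; A small random Z offset each frame makes the marker jitter.
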(event EventBeginPlay
  (bind _outactors (Actor|GetAllActorsOfClass "/Game/JustDoIT/Blueprints/BP_JustDoITCorporation.BP_JustDoITCorporation_C"))
  (if true
    (Variables|Default|SetCorporation (Utilities|Array|Get(acopy) _outactors))))

(event Collision|EventActorBeginOverlap
  (params (OtherActor :type Actor%20Object%20Reference)))

(event EventTick
  (params (DeltaSeconds :type Float%20%28single-precision%29))
  (bind _top (Variables|Default|GetTop))
  (bind _bottom (Variables|Default|GetBottom))
  (bind _corporation (Variables|Default|GetCorporation))
  (bind _totalmoneyearned (Variables|/Script/JustDoIT.JustDoITCorporation|GetTotalMoneyEarned _corporation))
  (bind _returnvalue (/ _totalmoneyearned 6e+03))
  (bind _returnvalue_2 (Math|Vector|Lerp(Vector) _bottom _top _returnvalue))
  (bind (_x _y _z) (Math|Vector|BreakVector _returnvalue_2))
  (if (Utilities|IsValid (Variables|Default|GetCorporation))
    (Transformation|SetWorldLocation (Variables|Default|GetParticleSystem) (Math|Vector|MakeVector _x _y (+ _z (Math|Random|RandomFloatinRange -3.0 3.0))) false)))

(fn ConstructionScript)