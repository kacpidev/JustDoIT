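; BP_JustDoITHUD is the HUD for JustDoIT that shows the gameplay widget and keeps a game timer.
; BeginPlay creates UMG_Gameplay for the owning player and adds it to the viewport, but sets GamePlayWidget to None rather than the new widget.
; Tick accumulates delta seconds into MyTimer while InGamePlay is true and GameEnded is false.
; The DrawGamePlayHUD event is an empty stub.
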(event EventBeginPlay
  (bind _returnvalue (UserInterface|CreateWidget "/Game/JustDoIT/UMG/UMG_GamePlay.UMG_Gameplay_C" (Game|Player|GetOwningPlayerController)))
  (UserInterface|Viewport|AddtoViewport _returnvalue 0)
  (Variables|Default|SetGamePlayWidget 0))

(event EventDrawGamePlayHUD)

(event EventTick
  (params (DeltaSeconds :type Float%20%28single-precision%29))
  (if (and (Variables|Default|GetbInGamePlay) (not (Variables|Default|GetbGameEnded)))
    (Variables|Default|SetMyTimer (+ DeltaSeconds (Variables|Default|GetMyTimer)))))

(fn ConstructionScript)