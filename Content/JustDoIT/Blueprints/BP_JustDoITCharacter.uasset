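; BP_JustDoITCharacter is a character Blueprint that shows the tool held in the left hand.
; The UpdateLeftTool event compares the integer ToolTypeL against E_ProblemType values and sets LeftHandMesh to the matching cable, floppy or CD-ROM mesh.
; Other values leave the mesh unchanged, the cable branch prints a debug string, and the construction script is empty.
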(event EventUpdateLeftTool
  (bind _lefthandmesh (Variables|Default|GetleftHandMesh))
  (if (== (Variables|Default|GetToolTypeL) (Math|Conversions|ToInteger(Byte) (Utilities|Enum|LiteralenumE_ProblemType "VE_NoCable")))
    (Development|PrintString 0 "Left update")
    (Components|StaticMesh|SetStaticMesh _lefthandmesh (Variables|Default|GetCable))
    (elif (== (Variables|Default|GetToolTypeL) (Math|Conversions|ToInteger(Byte) (Utilities|Enum|LiteralenumE_ProblemType "VE_NoOS")))
      (Components|StaticMesh|SetStaticMesh _lefthandmesh (Variables|Default|GetFloppy))
      (elif (== (Variables|Default|GetToolTypeL) (Math|Conversions|ToInteger(Byte) (Utilities|Enum|LiteralenumE_ProblemType "VE_BrokenCdRom")))
        (Components|StaticMesh|SetStaticMesh _lefthandmesh (Variables|Default|GetCdrom))))))

(fn ConstructionScript)