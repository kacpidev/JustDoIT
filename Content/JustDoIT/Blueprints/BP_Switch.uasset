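; BP_Switch is an interactable flip switch that toggles its ActorState on interaction.
; Player look-at turns custom depth and a raised translucent sort priority on or off for both meshes.
; Tick polls ActorState to tilt the switch, set the dynamic material's "on" parameter and update Rotated as its inverse.
; The construction script creates that material from M_Switch and sets ProblemType to NoObjectRequired.
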(event EventOnFinishPlayerLookat
  (bind _flip_switch (Variables|Default|Getflip_switch))
  (bind _staticmesh (Variables|Default|GetStaticMesh))
  (Rendering|SetRenderCustomDepth _flip_switch false)
  (Rendering|SetTranslucentSortPriority _flip_switch 0)
  (Rendering|SetRenderCustomDepth _staticmesh false)
  (Rendering|SetTranslucentSortPriority _staticmesh 0))

(event EventOnStartPlayerLookat
  (bind _flip_switch (Variables|Default|Getflip_switch))
  (bind _staticmesh (Variables|Default|GetStaticMesh))
  (Rendering|SetRenderCustomDepth _flip_switch true)
  (Rendering|SetTranslucentSortPriority _flip_switch 1000)
  (Rendering|SetRenderCustomDepth _staticmesh true)
  (Rendering|SetTranslucentSortPriority _staticmesh 1000))

(event EventTick
  (params (DeltaSeconds :type Float%20%28single-precision%29))
  (bind _actorstate (Variables|Default|GetActorState))
  (Rendering|Material|SetScalarParameterValue (Variables|Default|GetMaterialInstance) "on" (Math|Conversions|ToFloat(Boolean) _actorstate) :!class /Script/Engine.MaterialInstanceDynamic)
  (if (Math|Boolean|Equal(Boolean) _actorstate false)
    (Transformation|SetRelativeRotation (Variables|Default|Getflip_switch) "0, 0,-10.000000" false)
    (else
      (Transformation|SetRelativeRotation (Variables|Default|Getflip_switch) "0, 0,10.000000" false)))
  (Variables|Default|SetRotated (not _actorstate)))

(event EventOnInteraction
  (params (ProblemType :type Integer%20%28by%20ref%29))
  (Variables|Default|SetActorState (not (Variables|Default|GetActorState))))

(fn ConstructionScript
  (|CallParentFunction)
  (Variables|Default|SetProblemType (Math|Conversions|ToInteger(Byte) (Utilities|Enum|LiteralenumE_ProblemType "VE_NoObjectRequired")))
  (bind _returnvalue (Rendering|Material|CreateDynamicMaterialInstance (Variables|Default|Getflip_switch) 0 "/Game/JustDoIT/Materials/M_Switch.M_Switch" :!class /Script/Engine.PrimitiveComponent))
  (Variables|Default|SetMaterialInstance _returnvalue))